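; AI bot character for a shooter with kill scoring: it gets a random name, fires projectiles and respawns after death.
; StartShooting and StopShooting control a looping timer that spawns AIProj_BP at an arrow component.
; Damage updates a health widget that yaws toward the player.
; At zero health, a DoOnce credits the killing bot or player, drops the bot below the map, then respawns it at a random SpawnPoint with 100 health.
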(event `self.ReceiveBeginPlay`
  ; Begin_Play
  (set `self.Name` (`KismetTextLibrary.Conv_StringToText` (`KismetStringLibrary.Concat_StrStr` "Bot#: " (`KismetStringLibrary.Conv_IntToString` (`KismetMathLibrary.RandomInteger` 500)))))
  (bind _outactors (`GameplayStatics.GetAllActorsOfClass` "/Game/Spawner/SpawnPoint.SpawnPoint_C"))
  (set `self.SpawnPoints` _outactors)
  (bind _asai_w (cast `/Game/AI/AI_W` (`WidgetComponent.GetUserWidgetObject` (`self.Widget`))))
  (set `self.As AI W` _asai_w))

(event `self.ReceiveTick`
  (params (DeltaSeconds :type "Float (single-precision)"))
  (bind _widget (`self.Widget`))
  (bind (_returnvalue_roll _returnvalue_pitch _returnvalue_yaw) (`KismetMathLibrary.BreakRotator` (`KismetMathLibrary.FindLookAtRotation` (`SceneComponent.K2_GetComponentLocation` _widget) (`self.K2_GetActorLocation` (`GameplayStatics.GetPlayerCharacter` 0)))))
  ; Tick Widget Rotation
  (`SceneComponent.K2_SetWorldRotation` _widget (`KismetMathLibrary.MakeRotator` 0.0 0.0 _returnvalue_yaw) false false))

(event `AIHealthBonus`
  (params (MaxHealth :type "Float (double-precision)"))
  ; Health Bonus
  (bind _output_get (set `self.MaxHealth` MaxHealth))
  (set `self.Health` _output_get)
  (`/Game/AI/AI_W.SetHealth` (`self.As AI W`) (`self.Health`) (`self.MaxHealth`)))

(event `AddScore`
  (params (Value :type Integer))
  ; AddScore
  (set `self.Score` (+ (`self.Score`) Value)))

(event `Respawn`
  (bind _spawnpoints (`self.SpawnPoints`))
  ; Respawn
  (`KismetSystemLibrary.Delay` 0.2)
  (set `self.Health` 100.0)
  (`self.K2_SetActorLocation` (`self.K2_GetActorLocation` (`|GetArrayItem` _spawnpoints (`KismetMathLibrary.RandomIntegerInRange` 0 (- (`KismetArrayLibrary.Array_Length` _spawnpoints) 1)))) false true)
  (`/Game/AI/AI_W.SetHealth` (`self.As AI W`) (`self.Health`) (`self.MaxHealth`))
  (`self.ResetDoOnce`))

(event `StartShooting`
  ; Projectile
  (`KismetSystemLibrary.K2_SetTimer` null "AIShoot" (`self.RateofFire`) true))

(event `self.ReceiveAnyDamage`
  (params (Damage :type "Float (single-precision)") (DamageType :type "DamageType Object Reference") (InstigatedBy :type "Controller Object Reference") (DamageCauser :type "Actor Object Reference"))
  ; Health and Damage
  (set `self.Damage Causer` DamageCauser)
  (set `self.Health` (- (`self.Health`) Damage))
  (`self.CheckHealth`)
  (`/Game/AI/AI_W.SetHealth` (`self.As AI W`) (`self.Health`) (`self.MaxHealth`)))

(event `CheckHealth`
  (bind _damage_causer (`self.Damage Causer`))
  ; Health and Damage
  (if (<= (`self.Health`) 0.0)
    (`/Engine/EditorBlueprintResources/StandardMacros.DoOnce` false :!label _label
      (:`Completed`
        (bind _asaichar_bp (cast `/Game/AI/AIChar_BP` _damage_causer)
          (:`then`
            (`self.AddScore` _asaichar_bp 1))
          (:`CastFailed`
            (bind _asplayer_char_bp (cast `/Game/Player/PlayerChar_BP` _damage_causer))
            (`/Game/Player/PlayerChar_BP.AddScore` _asplayer_char_bp 1)))
        (`self.K2_SetActorLocation` (0.0 0.0 -5000.0))
        (`self.Respawn`)))))

(event `ResetDoOnce`
  ; Health and Damage
  (goto _label :!via `Reset`))

(event `StopShooting`
  ; Projectile
  (`KismetSystemLibrary.K2_ClearTimer` null "AIShoot"))

(event `HealthBonus`
  (params (MaxHealth :type "Float (double-precision)"))
  ; Health and Damage
  (bind _output_get (set `self.MaxHealth` MaxHealth))
  (set `self.Health` _output_get))

(event `AIShoot`
  ; Projectile
  ;; Spawn Projectiles
  (`|SpawnActorFromClass` "/Game/AI/AIProj_BP.AIProj_BP_C" (`SceneComponent.K2_GetComponentToWorld` (`self.Arrow1`)) "Undefined" "MultiplyWithRoot" self null))

(fn `UserConstructionScript`)