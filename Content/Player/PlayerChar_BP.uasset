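; Player character Blueprint with movement, look and jump input, projectile firing and a simple health and respawn loop.
; Fire spawns PlayerProj_BP at the Arrow1 component's transform with the character as owner.
; Damage reduces Health and runs CheckHP, which at zero or below restores Health and teleports the character to a random SpawnPoint cached at BeginPlay.
; HealthBonus sets Health to a supplied maximum; the CheckHealth function is empty.
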(event `self.ReceiveBeginPlay`
  (bind _outactors (`GameplayStatics.GetAllActorsOfClass` "/Game/Spawner/SpawnPoint.SpawnPoint_C"))
  (set `self.SpawnPoints` _outactors))

(event `Respawn`
  (bind _spawnpoints (`self.SpawnPoints`))
  (set `self.Health` 100.0)
  (`self.K2_SetActorLocation` (`self.K2_GetActorLocation` (`|GetArrayItem` _spawnpoints (`KismetMathLibrary.RandomIntegerInRange` 0 (- (`KismetArrayLibrary.Array_Length` _spawnpoints) 1)))) false true))

(event `InputAxis|MoveForward`
  (params (AxisValue :type "Float (single-precision)"))
  (bind (_returnvalue_roll _returnvalue_pitch _returnvalue_yaw) (`KismetMathLibrary.BreakRotator` (`self.GetControlRotation`)))
  ; Character Movement
  (`self.AddMovementInput` (`KismetMathLibrary.GetForwardVector` (`KismetMathLibrary.MakeRotator` 0.0 0.0 _returnvalue_yaw)) AxisValue))

(event `InputAxis|MoveRight`
  (params (AxisValue :type "Float (single-precision)"))
  (bind (_returnvalue_roll _returnvalue_pitch _returnvalue_yaw) (`KismetMathLibrary.BreakRotator` (`self.GetControlRotation`)))
  ; Character Movement
  (`self.AddMovementInput` (`KismetMathLibrary.GetRightVector` (`KismetMathLibrary.MakeRotator` _returnvalue_roll 0.0 _returnvalue_yaw)) AxisValue))

(event `InputAxis|LookUp`
  (params (AxisValue :type "Float (single-precision)"))
  ; Character Movement
  (`self.AddControllerPitchInput` AxisValue))

(event `InputAxis|Turn`
  (params (AxisValue :type "Float (single-precision)"))
  ; Character Movement
  (`self.AddControllerYawInput` AxisValue))

(event `InputAction|Jump`
  (params (Key :type "Key Structure"))
  ; Character Movement
  (:`Pressed`
    (`self.Jump`))
  (:`Released`
    (`self.StopJumping`)))

(event `InputAction|Fire`
  (params (Key :type "Key Structure"))
  ; Fire Event
  (:`Pressed`
    (`|SpawnActorFromClass` "/Game/Player/PlayerProj_BP.PlayerProj_BP_C" (`SceneComponent.K2_GetComponentToWorld` (`self.Arrow1`)) "Undefined" "MultiplyWithRoot" self null)))

(event `self.ReceiveAnyDamage`
  (params (Damage :type "Float (single-precision)") (DamageType :type "DamageType Object Reference") (InstigatedBy :type "Controller Object Reference") (DamageCauser :type "Actor Object Reference"))
  ; Health and Damage
  (set `self.Damage Causer` DamageCauser)
  (set `self.Health` (- (`self.Health`) Damage))
  (`self.CheckHP`)
  (`KismetSystemLibrary.PrintString` (`KismetStringLibrary.Conv_DoubleToString` (`self.Health`))))

(event `CheckHP`
  ; Health and Damage
  (if (<= (`self.Health`) 0.0)
    (`self.Respawn`)))

(event `HealthBonus`
  (params (MaxHealth :type "Float (double-precision)"))
  ; Health and Damage
  (bind _output_get (set `self.MaxHealth` MaxHealth))
  (set `self.Health` _output_get))

(fn `CheckHealth`)

(fn `UserConstructionScript`)