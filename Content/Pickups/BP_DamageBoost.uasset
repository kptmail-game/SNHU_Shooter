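; BP_DamageBoost is a pickup that raises the player character's damage when its AddBonus event fires.
; It casts the player to PlayerChar_BP, sets DamageAmount to a fixed boosted value, starts a translucent blue camera fade and destroys itself.
; A delayed branch that would restore damage and run a second fade is disconnected, so this Blueprint never reverts the boost.
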(event `self.AddBonus`
  (params (Player :type "/Game/Player/PlayerChar_BP Object Reference") (AI :type "/Game/AI/AIChar_BP Object Reference"))
  (`/Engine/EditorBlueprintResources/StandardMacros.IsValid` Player
    (:`Is Valid`
      (bind _asplayer_char_bp (cast `/Game/Player/PlayerChar_BP` Player))
      (set `/Game/Player/PlayerChar_BP.DamageAmount` 100.0 _asplayer_char_bp)
      (`PlayerCameraManager.StartCameraFade` (`GameplayStatics.GetPlayerCameraManager` 0) 0.0 0.3 5.0 (struct :`G` 0.049468 :`B` 1.0 :`A` 1.0) false false)
      (`self.K2_DestroyActor`))))

(fn `UserConstructionScript`
  (`parent.UserConstructionScript`))